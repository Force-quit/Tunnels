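; BP_DifficultyLight is a lighting actor whose look shifts over the course of play, its name suggesting a cue for rising difficulty.
; Each tick it lowers the color temperature of two directional lights by a fixed delta and pitches the actor by a steadily growing rotation speed.
; Changes are per frame, not scaled by delta time.
; A Stop event, meant for player death, disables the tick to freeze the lighting.
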(event Custom|Stop
  ;[1 1 1] Player died
  (Actor|Tick|SetActorTickEnabled false))

(event EventTick
  (params (DeltaSeconds :type Float%20%28single-precision%29))
  (bind _directionallight2 (Variables|Default|GetDirectionalLight2))
  (bind _directionallight (Variables|Default|GetDirectionalLight))
  ;[1 1 1] Lower temperature with time
  (Class|LightComponent|SetTemperature _directionallight (- (Variables|/Script/Engine.LightComponent|GetTemperature _directionallight) (Variables|Default|GetdeltaTemperature)))
  (Class|LightComponent|SetTemperature _directionallight2 (- (Variables|/Script/Engine.LightComponent|GetTemperature _directionallight2) (Variables|Default|GetdeltaTemperature)))
  (bind _output_get (Variables|Default|SetrotationSpeed (+ (Variables|Default|GetrotationSpeed) (Variables|Default|GetrotationSpeedIncrement))))
  (Class|Actor|AddActorWorldRotation (Math|Rotator|MakeRotator 0.0 _output_get 0.0)))

(fn ConstructionScript)