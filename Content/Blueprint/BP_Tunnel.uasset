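; Endless tunnel segment that moves along world Y at a periodically increasing speed, carrying child laser obstacles.
; When BP_Character leaves EndTrigger, it teleports by tunnel count times its length, recycling itself instead of respawning.
; Each recycle restores cached laser transforms, then randomly disables or rotates each laser (random offset has zero weight).
; A timer lowers the removal chance for denser lasers; StopMoving halts timers, movement and rotation.
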(event OnComponentEndOverlap(EndTrigger)
  (params (OverlappedComponent :type Primitive%20Component%20Object%20Reference) (OtherActor :type Actor%20Object%20Reference) (OtherComp :type Primitive%20Component%20Object%20Reference) (OtherBodyIndex :type Integer))
  (bind _returnvalue (Transformation|GetActorLocation))
  ;[1 1 1] End trigger overlap
  (Utilities|Casting|CastToBP_Character OtherActor)
  (Transformation|SetActorLocation (Math|Vector|MakeVector (.x _returnvalue) (+ (.y _returnvalue) (Variables|Default|GetrelocationOffset)) (.z _returnvalue)) false true)
  (for (_array_element _array_index) (Variables|Default|GetlaserReferences)
    (Transformation|SetRelativeTransform (Variables|/Game/Blueprint/BP_Laser.BP_Laser_C|GetRoot _array_element) (Utilities|Array|Get(acopy) (Variables|Default|GetlasersInitialTransform) _array_index) false true))
  (CallFunction|PrepareTunnel))

(event Custom|Prepare%20Tunnel
  ;[1 1 1] Prepare tunnel
  (for _array_element (Variables|Default|GetlaserReferences)
    (if (Math|Random|RandomBoolwithWeight (Variables|LaserParameters|GetremoveLaserWeight))
      (Default|Disable _array_element)
      (else
        (Default|Enable _array_element)
        (CallFunction|RelocateLaser _array_element)))))

(event Custom|SpeedUp
  ;[1 1 1] Speed Up
  (Variables|Default|SetmovingSpeed (+ (Variables|Default|GetmovingSpeedIncrement) (Variables|Default|GetmovingSpeed))))

(event Custom|Relocate%20laser
  (params (laserComponent :type BP%20Laser%20Object%20Reference))
  (bind _maxlasertranslation (Variables|LaserParameters|GetmaxLaserTranslation))
  ;[1 1 1] Relocate lasers
  (Transformation|AddActorLocalRotation laserComponent (Math|Rotator|MakeRotator 0.0 (Math|Random|RandomFloatinRange 0.0 (Variables|LaserParameters|GetmaxLaserRotation)) 0.0) false false)
  (if (Math|Random|RandomBoolwithWeight 0.0)
    (bind _result (Math|Float|NegateFloat _maxlasertranslation)
      (:%20%20
        (Transformation|AddActorLocalOffset laserComponent (Math|Vector|MakeVector (Math|Random|RandomFloatinRange _result _maxlasertranslation) 0.0 (Math|Random|RandomFloatinRange _result _maxlasertranslation)) false true)))))

(event Custom|StartMoving
  ;[1 1 1] Start moving
  (Actor|Tick|SetActorTickEnabled true)
  (bind _returnvalue (Utilities|Time|SetTimerbyEvent (delegate Custom|SpeedUp) (Variables|Default|GetmovingSpeedUpdateFrequence) true)))

(event Custom|StopMoving
  ;[1 1 1] Player died
  (Utilities|Time|ClearandInvalidateTimerbyHandle (stale Custom|StartMoving _returnvalue))
  (Utilities|FlowControl|Sequence
    (:then_0
      ;[1 1 1] Gradually spawn more lasers
      (Utilities|Time|ClearandInvalidateTimerbyHandle (stale EventBeginPlay _returnvalue)))
    (:then_1
      (Actor|Tick|SetActorTickEnabled false)
      (Components|Activation|Deactivate (Variables|Default|GetRotatingMovement)))))

(event Custom|GraduallySpawnMoreLasers
  ;[1 1 1] Gradually spawn more lasers
  (bind _output_get (Variables|LaserParameters|SetremoveLaserWeight (- (Variables|LaserParameters|GetremoveLaserWeight) 0.02)))
  (if (<= _output_get 0.0)
    (Variables|LaserParameters|SetremoveLaserWeight 0.0)
    (Utilities|Time|ClearandInvalidateTimerbyHandle (stale EventBeginPlay _returnvalue))))

(event EventBeginPlay
  ;[1 1 1] BeginPlay
  (Utilities|FlowControl|Sequence
    (:then_0
      (for _array_element (Actor|GetAllChildActors false)
        (bind _asbp_laser (Utilities|Casting|CastToBP_Laser _array_element))
        (Utilities|Array|Add (Variables|Default|GetlaserReferences) _asbp_laser)
        (Utilities|Array|Add (Variables|Default|GetlasersInitialTransform) (Transformation|GetRelativeTransform (Variables|/Game/Blueprint/BP_Laser.BP_Laser_C|GetRoot _asbp_laser))))
      (CallFunction|PrepareTunnel)
      ;[1 1 1] Gradually spawn more lasers
      (bind _returnvalue (Utilities|Time|SetTimerbyEvent (delegate Custom|GraduallySpawnMoreLasers) 1e+01 true)))
    (:then_1
      (bind _outactors (Actor|GetAllActorsOfClass "BP_Tunnel_C"))
      (Variables|Default|SetrelocationOffset (* (Math|Conversions|ToFloat(Integer) (Utilities|Array|Length _outactors)) (* (.y (.BoxExtent (Collision|GetActorBounds false false))) 2.0))))))

(event EventTick
  (params (DeltaSeconds :type Float%20%28single-precision%29))
  ;[1 1 1] Continuous forward movement
  (Transformation|AddActorWorldOffset (Math|Vector|MakeVector 0.0 (Variables|Default|GetmovingSpeed) 0.0)))

(fn ConstructionScript)