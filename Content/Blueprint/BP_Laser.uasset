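; BP_Laser is a laser hazard actor that kills any BP_Character overlapping its capsule.
; A Niagara system draws the beam, with its end set on BeginPlay from the capsule's scaled height along negative Z.
; SetLaserWidth drives both the beam width and the capsule radius, scaled down by 100.
; Enable and Disable toggle visibility, query collision and overlap events together.
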(event OnComponentBeginOverlap(Capsule)
  (params (OverlappedComponent :type Primitive%20Component%20Object%20Reference) (OtherActor :type Actor%20Object%20Reference) (OtherComp :type Primitive%20Component%20Object%20Reference) (OtherBodyIndex :type Integer) (bFromSweep :type Boolean) (SweepResult :type Hit%20Result%20Structure%20%28by%20ref%29))
  ;[1 1 1] Hit player
  (bind _asbp_character (Utilities|Casting|CastToBP_Character OtherActor))
  (Default|Die _asbp_character))

(event Custom|Disable
  (bind _capsule (Variables|Default|GetCapsule))
  ;[1 1 1] Enable/Disable laser
  (Rendering|SetActorHiddenInGame true)
  (Collision|SetCollisionEnabled _capsule "NoCollision")
  (Variables|/Script/Engine.PrimitiveComponent|SetbGenerateOverlapEvents _capsule false))

(event Custom|Enable
  (bind _capsule (Variables|Default|GetCapsule))
  ;[1 1 1] Enable/Disable laser
  (Rendering|SetActorHiddenInGame false)
  (Collision|SetCollisionEnabled _capsule "QueryOnly")
  (Variables|/Script/Engine.PrimitiveComponent|SetbGenerateOverlapEvents _capsule true))

(event Custom|SetLaserWidth
  (params (newWidth :type Float%20%28double-precision%29))
  ;[1 1 1] Set laser width
  (Niagara|SetNiagaraVariable(Float) (Variables|Default|GetNE_Laser_System) "BeamWidth" newWidth)
  (Components|Capsule|SetCapsuleRadius (Variables|Default|GetCapsule) (/ newWidth 1e+02) false))

(event EventBeginPlay
  ;[1 1 1] Set beam end
  (Class|NiagaraComponent|SetNiagaraVariableVec3 (Variables|Default|GetNE_Laser_System) "Beamend" (Math|Vector|MakeVector 0.0 0.0 (* -2.0 (Components|Capsule|GetScaledCapsuleHalfHeight (Variables|Default|GetCapsule))))))

(fn ConstructionScript)